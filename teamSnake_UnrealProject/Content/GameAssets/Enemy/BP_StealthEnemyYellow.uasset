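; BP_StealthEnemyYellow is a stealth AI enemy that shoots water projectiles at the player.
; FireGun plays a shoot montage whose notify spawns a projectile, bound to DamagePlayer for damage and splash effects on player hits.
; Death plays a damaged montage, shows ZZZ and disables capsule collision.
; Construction applies the variant mesh and AnimBP, while functions supply patrol route, ideal range and movement speeds.
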(event `self.ReceiveBeginPlay`
  (bind _asaic_stealth (cast `/Game/GameAssets/Enemy/AI/AIC_Stealth` (`AIBlueprintHelperLibrary.GetAIController` self)))
  (set `self.AIC Stealth` _asaic_stealth))

(event `FireGun`
  ;[1 1 1] Comment
  (`|PlayMontage` (`self.Mesh`) "/Game/GameAssets/Enemy/Animations/EnemyKid_Shoot_Montage.EnemyKid_Shoot_Montage"
    (:`then`
      (`self.OnAttackEnd` :!label _label))
    (:`OnCompleted`
      (goto _label))
    (:`OnNotifyBegin`
      (`GameplayStatics.PlaySound2D` "/Game/GameAssets/Sound_Effects/watershot_liamEdit.watershot_liamEdit" 1.0 1.0 0.0 null null)
      (bind _returnvalue (`|SpawnActorFromClass` "/Game/GameAssets/Blueprints/Projectiles/BP_ProjectileEnemy.BP_ProjectileEnemy_C" (`SceneComponent.K2_GetComponentToWorld` (`self.Launchpoint`)) "Undefined" "MultiplyWithRoot" self null))
      (add `/Game/GameAssets/Blueprints/Projectiles/BP_ProjectileEnemy.OnProjectileImpact` _returnvalue (delegate `Damage Player`))
      (`PrimitiveComponent.IgnoreActorWhenMoving` (`self.CapsuleComponent`) null true))))

(event `Damage Player`
  (params (OtherActor :type "Actor Object Reference") (HitResult :type "HitResult Structure"))
  (bind (_bblockinghit _binitialoverlap _time _distance _location _impactpoint _normal _impactnormal _physmat _hitactor) (`GameplayStatics.BreakHitResult` HitResult))
  ;[1 1 1] Handles Damage Events on Players when a projectile hits the player
  (if (== (`GameplayStatics.GetPlayerCharacter` 0) _hitactor)
    (bind _returnvalue (`AddComponent|NODE_AddBPC_GabesDamageImplementation-0` :`self` OtherActor))
    (`/Game/GameAssets/Blueprints/DamageSystem/BPC_GabesDamageImplementation.Handle Damage` _returnvalue "NewEnumerator2" -4 null)
    (`NiagaraFunctionLibrary.SpawnSystemAtLocation` "/Game/OtherVFX/Waterburst2.Waterburst2" _impactpoint)
    (`GameplayStatics.PlaySoundAtLocation` "/Game/GameAssets/Sound_Effects/damagesting.damagesting" _impactpoint (struct) 1.0 1.0 0.0 null null null null)))

(event `Death`
  (`|PlayMontage` (`self.Mesh`) "/Game/GameAssets/Enemy/Animations/EnemyKid_Damaged_Montage.EnemyKid_Damaged_Montage"
    (:`then`
      (`SceneComponent.SetVisibility` (`self.ZZZ`) true false)
      (`PrimitiveComponent.SetCollisionEnabled` (`self.CapsuleComponent`) "NoCollision"))))

(fn `GetIdealRange`
  (returns (AttackRadius :type "Float (double-precision)"))
  (return 500.0))

(fn `GetPatrolRoute`
  (returns (PatrolRoute :type "/Game/GameAssets/Enemy/AI/BP_PatrolRoute Object Reference"))
  (return (`self.PatrolRoute`)))

(fn `SetMovementState`
  (params (Speed :type "/Game/GameAssets/Enemy/AI/Enums/E_MovementState Enum" :default "NewEnumerator0"))
  (returns (SpeedValue :type "Float (double-precision)"))
  (bind _output_get (set `CharacterMovementComponent.MaxWalkSpeed` (select `/Game/GameAssets/Enemy/AI/Enums/E_MovementState` Speed :`NewEnumerator0` 150.0 :`NewEnumerator1` 400.0 :!type "Float (single-precision)") (`self.CharacterMovement`)))
  (return _output_get))

(fn `UserConstructionScript`
  (`SkeletalMeshComponent.SetSkeletalMeshAsset` (`self.Mesh`) (`self.EnemyVariant`))
  (`SkeletalMeshComponent.SetAnimInstanceClass` (`self.Mesh`) (`self.Enemy_AnimBP`)))