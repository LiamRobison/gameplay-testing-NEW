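; Damage system component that tracks health, death and invincibility for its owner and reports whether a hit took effect.
; TakeDamage uses the CanBeDamaged branch to reject hits when dead or invincible, though the ShouldBeInvincible flag in DamageInfo bypasses invincibility.
; Accepted hits reduce health, then fire OnDeath at zero or below, or OnDamageResponse when interruptible or forced.
; Non-lethal, non-interrupting hits still deduct health but have no explicit return value.
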(event `self.ReceiveBeginPlay`)

(fn `TakeDamage`
  (params (DamageInfo :type "/Game/GameAssets/Blueprints/DamageSystem/S_DamageInfo Structure"))
  (returns (WasDamaged :type Boolean))
  (bind (_amount _damagetype _damageresponse _shouldbeinvincible_ _shouldinterupt_) (break `/Game/GameAssets/Blueprints/DamageSystem/S_DamageInfo` DamageInfo))
  (`self.CanBeDamaged` _shouldbeinvincible_
    (:`DoDamage`
      (bind _output_get (set `self.CurrentHealth` (- (`self.CurrentHealth`) _amount)))
      (if (<= _output_get 0)
        (set `self.IsDead?` true)
        (`self.OnDeath`)
        (return true)
        (elif (or (`self.IsInterupible?`) _shouldinterupt_)
          (`self.OnDamageResponse` _damageresponse)
          (return true))))
    (:`NoDamage`
      (return false))))