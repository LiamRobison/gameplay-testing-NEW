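; Damage component that applies hits and handles death for the player and stealth AI enemies, branching on target actor type.
; HandleDamage kills enemies outright regardless of damage amount, while player damage is passed to the character's UpdateCurrentHealth.
; HandleDeath ragdolls the target: enemies also stop AI logic, enter dead state and end their alert through the game mode, while the player loses input.
; BeginPlay caches the player character and game mode.
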(event `self.ReceiveBeginPlay`
  (bind _asbp_third_person_character (cast `/Game/GameAssets/Blueprints/BP_ThirdPersonCharacter` (`GameplayStatics.GetPlayerCharacter` 0)))
  (set `self.As BP Third Person Character` _asbp_third_person_character)
  (bind _asbp_third_person_game_mode (cast `/Game/GameAssets/Blueprints/BP_ThirdPersonGameMode` (`GameplayStatics.GetGameMode`)))
  (set `self.As BP Third Person Game Mode` _asbp_third_person_game_mode))

(fn `Handle Damage`
  (params (`Target Actor Type` :type "/Game/GameAssets/Blueprints/DamageSystem/Enum_TargetActorType Enum" :default "NewEnumerator0") (`Enemy Actor Object Reference` :type "/Game/GameAssets/Enemy/BP_StealthEnemy Object Reference") (`Damage Taken` :type Integer))
  (switch `/Game/GameAssets/Blueprints/DamageSystem/Enum_TargetActorType` `Target Actor Type`
    (:`NewEnumerator0`
      (`self.Handle Death` "NewEnumerator0" `Enemy Actor Object Reference`))
    (:`NewEnumerator1`
      (`/Game/GameAssets/Blueprints/BP_ThirdPersonCharacter.Update Current Health` (`self.As BP Third Person Character`) `Damage Taken`))))

(fn `Handle Death`
  (params (`Target Actor Type` :type "/Game/GameAssets/Blueprints/DamageSystem/Enum_TargetActorType Enum" :default "NewEnumerator0") (`Actor Object Reference` :type "/Game/GameAssets/Enemy/BP_StealthEnemy Object Reference"))
  (locals (`Local Actor Object Reference` :type "/Game/GameAssets/Enemy/BP_StealthEnemy Object Reference"))
  (set `local.Local Actor Object Reference` `Actor Object Reference`)
  (switch `/Game/GameAssets/Blueprints/DamageSystem/Enum_TargetActorType` `Target Actor Type`
    (:`NewEnumerator0`
      (`/Engine/EditorBlueprintResources/StandardMacros.IsValid` (`local.Local Actor Object Reference`)
        (:`Is Valid`
          (`PrimitiveComponent.SetSimulatePhysics` (`Character.Mesh` (`local.Local Actor Object Reference`)) true)
          (`PrimitiveComponent.SetCollisionEnabled` (`Character.CapsuleComponent` (`local.Local Actor Object Reference`)) "QueryAndPhysics")
          (`BrainComponent.StopLogic` (`AIController.BrainComponent` (`/Game/GameAssets/Enemy/BP_StealthEnemy.AIC Stealth` (`local.Local Actor Object Reference`))) "")
          (`/Game/GameAssets/Enemy/AI/AIC_Stealth.SetDeadState` (`/Game/GameAssets/Enemy/BP_StealthEnemy.AIC Stealth` (`local.Local Actor Object Reference`)))
          (`/Game/GameAssets/Blueprints/BP_ThirdPersonGameMode.End Alert` (`self.As BP Third Person Game Mode`) (`local.Local Actor Object Reference`)))
        (:`Is Not Valid`
          (`KismetSystemLibrary.PrintString` "WARNING: ENEMY OBJECT REFERENCE NOT VALID IN DPC_DAMAGEIMPLEMENTATION.HANDLEDEATH" true true (struct :`G` 0.66 :`B` 1.0 :`A` 1.0) 100.0))))
    (:`NewEnumerator1`
      (`PrimitiveComponent.SetSimulatePhysics` (`Character.Mesh` (`self.As BP Third Person Character`)) true)
      (`PrimitiveComponent.SetCollisionEnabled` (`Character.Mesh` (`self.As BP Third Person Character`)) "QueryAndPhysics")
      (`Actor.DisableInput` (`self.As BP Third Person Character`) (`GameplayStatics.GetPlayerController` 0)))))