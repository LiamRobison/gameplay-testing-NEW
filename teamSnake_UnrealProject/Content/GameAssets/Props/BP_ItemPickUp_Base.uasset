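; Base item pickup that adds ammo for its PickUpType to the player character when touched.
; BeginPlay caches the player's BP_ThirdPersonCharacter, and sphere overlaps from that character look up the type in its EquipmentHandler map.
; Unless ammo reserve equals the maximum, it calls UpdateEquipment, destroys itself and prints a debug string.
; The pickup sound plays from the Destroyed event, so any destruction of the actor triggers it.
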(event `self.ReceiveBeginPlay`
  (bind _asbp_third_person_character (cast `/Game/GameAssets/Blueprints/BP_ThirdPersonCharacter` (`GameplayStatics.GetPlayerCharacter` 0)))
  (set `self.As BP Third Person Character` _asbp_third_person_character))

(event `self.Sphere.OnComponentBeginOverlap`
  (params (OverlappedComponent :type "PrimitiveComponent Object Reference") (OtherActor :type "Actor Object Reference") (OtherComp :type "PrimitiveComponent Object Reference") (OtherBodyIndex :type Integer) (bFromSweep :type Boolean) (SweepResult :type "HitResult Structure (by ref)"))
  (bind _as_bp_third_person_character (`self.As BP Third Person Character`))
  (bind _value (`BlueprintMapLibrary.Map_Find` (`/Game/GameAssets/Blueprints/BP_ThirdPersonCharacter.Equipment Handler` _as_bp_third_person_character) (`self.Pick-Up Type`)))
  (if (== OtherActor _as_bp_third_person_character)
    (if (not (== (`.AmmoMaxium_4_EBE89E0D46CA6C02275134BAB1655E21` (break `/Game/GameAssets/Blueprints/GameData/OBJ_Equipment` _value)) (`.AmmoReserve_6_6FEB56504AFBB495AACC21B046E6D345` (break `/Game/GameAssets/Blueprints/GameData/OBJ_Equipment` _value))))
      (`/Game/GameAssets/Blueprints/BP_ThirdPersonCharacter.UpdateEquipment` _as_bp_third_person_character (`self.Pick-Up Type`) (`self.+/- 1x Ammo`))
      (`self.K2_DestroyActor`)
      (`KismetSystemLibrary.PrintString` "Hello"))))

(event `self.ReceiveDestroyed`
  (`GameplayStatics.PlaySound2D` (`self.Pickup_Sound`) 1.0 1.0 0.0 null null))

(fn `UserConstructionScript`)