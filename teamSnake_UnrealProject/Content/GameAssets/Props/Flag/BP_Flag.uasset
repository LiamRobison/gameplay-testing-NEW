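; BP_Flag is a prop actor that the third-person player picks up by touching it.
; On BeginPlay it caches the player character and casts its owner to a stealth enemy.
; When the player overlaps its Box, the flag destroys itself.
; A disconnected node that would restart the owning enemy's AI brain logic never runs.
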(event `self.ReceiveBeginPlay`
  (bind _asbp_third_person_character (cast `/Game/GameAssets/Blueprints/BP_ThirdPersonCharacter` (`GameplayStatics.GetPlayerCharacter` 0)))
  (set `self.BP Third Person Character Ref` _asbp_third_person_character)
  (bind _asbp_stealth_enemy (cast `/Game/GameAssets/Enemy/BP_StealthEnemy` (`self.GetOwner`)))
  (set `self.BP Stealth Enemy Ref` _asbp_stealth_enemy))

(event `self.Box.OnComponentBeginOverlap`
  (params (OverlappedComponent :type "PrimitiveComponent Object Reference") (OtherActor :type "Actor Object Reference") (OtherComp :type "PrimitiveComponent Object Reference") (OtherBodyIndex :type Integer) (bFromSweep :type Boolean) (SweepResult :type "HitResult Structure (by ref)"))
  (if (== (`self.BP Third Person Character Ref`) OtherActor)
    (`self.K2_DestroyActor`)))

(fn `UserConstructionScript`)