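; Base player weapon Blueprint for a slingshot that fires projectiles and damages what they hit.
; Readying shows the mesh, while firing also plays a shoot montage and sound and spawns a BP_ProjectilePlayer at the launch point.
; The weapon binds to the projectile's impact event, sends fixed damage through an interface message and spawns a water-burst effect when that succeeds.
; CombatResult is an unfinished hit-check helper with disconnected enemy-check logic.
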(event `ReadyWeapon`
  (`SceneComponent.SetVisibility` (`self.StaticMesh`) true false))

(event `FireWeapon`
  (`SceneComponent.SetVisibility` (`self.StaticMesh`) true false)
  (`|PlayMontage` null "/Game/GameAssets/Props/Weapons/Slingshot/Animations/SlingShotRig_Shoot_Anim_Montage.SlingShotRig_Shoot_Anim_Montage"
    (:`then`
      (`GameplayStatics.PlaySound2D` "/Game/GameAssets/Sound_Effects/slingfire2.slingfire2" 1.0 1.0 0.0 null null)
      (bind _returnvalue (`|SpawnActorFromClass` "/Game/GameAssets/Blueprints/Projectiles/BP_ProjectilePlayer.BP_ProjectilePlayer_C" (`SceneComponent.K2_GetComponentToWorld` (`self.LaunchPoint_ref`)) "Undefined" "MultiplyWithRoot" self null))
      (add `/Game/GameAssets/Blueprints/Projectiles/BP_ProjectilePlayer.OnProjectileImpact` _returnvalue (delegate `DamageEnemy`)))))

(event `DamageEnemy`
  (params (OtherActor :type "Actor Object Reference") (HitResult :type "HitResult Structure"))
  (bind _wasdamaged (message `/Game/GameAssets/Blueprints/DamageSystem/BPI_Damagable.TakeDamage` OtherActor (make `/Game/GameAssets/Blueprints/DamageSystem/S_DamageInfo` 5 "NewEnumerator1")))
  (if _wasdamaged
    (`NiagaraFunctionLibrary.SpawnSystemAtLocation` "/Game/OtherVFX/Waterburst2.Waterburst2" (`.ImpactPoint` (`GameplayStatics.BreakHitResult` HitResult)))))

(fn `CombatResult`
  (params (`Out Hit` :type "HitResult Structure") (`Return Value` :type Boolean))
  (returns (`Out Actor` :type "Actor Object Reference"))
  (if `Return Value`
    (set `self.HitActor` (`.HitActor` (`GameplayStatics.BreakHitResult` `Out Hit`)))
    (return null)))

(fn `UserConstructionScript`)