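; Base Blueprint for player weapons, providing ReadyWeapon and FireWeapon events.
; FireWeapon spawns a BP_ProjectileTest actor at the Scene component's world transform, while ReadyWeapon is empty.
; An unconnected hitscan draft line-traces from the player character along its forward vector by Range and prints hit enemies found through an IsEnemy interface message.
; CombatResult only extracts the hit actor; its enemy check is also unconnected.
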(event `ReadyWeapon`)

(event `FireWeapon`
  (`|SpawnActorFromClass` "/Game/GameAssets/Props/Weapons/PlayerWeapons/BP_ProjectileTest.BP_ProjectileTest_C" (`SceneComponent.K2_GetComponentToWorld` (`self.Scene`)) "Undefined" "MultiplyWithRoot" null null))

(fn `CombatResult`
  (params (`Out Hit` :type "HitResult Structure") (`Return Value` :type Boolean))
  (returns (`Out Actor` :type "Actor Object Reference"))
  (if `Return Value`
    (set `self.HitActor` (`.HitActor` (`GameplayStatics.BreakHitResult` `Out Hit`)))
    (return null)))

(fn `UserConstructionScript`)